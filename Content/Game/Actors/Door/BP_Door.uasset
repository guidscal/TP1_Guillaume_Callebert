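; Interactable door actor that swings open and closed on Interact, with a sound for each direction.
; An IsOpen flag toggles playing or reversing the OpenCloseDoor timeline, whose Alpha lerps the door mesh's relative yaw between shut and open.
; A sphere collision shows the interaction prompt widget on overlap and hides it on exit, without filtering which actor overlaps.
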(event OnComponentBeginOverlap(SphereCollision)
  (params (OverlappedComponent :type Primitive%20Component%20Object%20Reference) (OtherActor :type Actor%20Object%20Reference) (OtherComp :type Primitive%20Component%20Object%20Reference) (OtherBodyIndex :type Integer) (bFromSweep :type Boolean) (SweepResult :type Hit%20Result%20Structure%20%28by%20ref%29))
  (Rendering|SetVisibility (Variables|Default|GetWidgetTextInteraction) true false))

(event OnComponentEndOverlap(SphereCollision)
  (params (OverlappedComponent :type Primitive%20Component%20Object%20Reference) (OtherActor :type Actor%20Object%20Reference) (OtherComp :type Primitive%20Component%20Object%20Reference) (OtherBodyIndex :type Integer))
  (Rendering|SetVisibility (Variables|Default|GetWidgetTextInteraction) false false))

(event EventBeginPlay
  (bind _aswbp_interaction (Utilities|Casting|CastToWBP_Interaction (UserInterface|GetUserWidgetObject (Variables|Default|GetWidgetTextInteraction))))
  (Variables|Default|SetWBP_Interaction_Ref _aswbp_interaction)
  (Rendering|SetVisibility (Variables|Default|GetWidgetTextInteraction) false false))

(event Collision|EventActorBeginOverlap
  (params (OtherActor :type Actor%20Object%20Reference)))

(event EventTick
  (params (DeltaSeconds :type Float%20%28single-precision%29)))

(event EventInteract
  (params (Actor :type Actor%20Object%20Reference))
  (if (Variables|Default|GetisOpen)
    (Variables|Default|SetisOpen false)
    (Audio|PlaySound2D "/Game/CustomContent/Sounds/Door/S_DoorClose_Cue.S_DoorClose_Cue" 1.0 1.0 0.0 0 0)
    (bind _alpha (Timeline|OpenCloseDoor Reverse)
      (:Update
        (Transformation|SetRelativeRotation (Variables|Default|GetSM_OpenableDoor) (Math|Rotator|MakeRotator 0.0 0.0 (Math|Float|Lerp 0.0 1.2e+02 _alpha)) false false)))
    (else
      (Variables|Default|SetisOpen true)
      (Audio|PlaySound2D "/Game/CustomContent/Sounds/Door/S_DoorOpen_Cue.S_DoorOpen_Cue" 1.0 1.0 0.0 0 0)
      (Timeline|OpenCloseDoor Play))))

(fn ConstructionScript)