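; Dynamite actor that, when interacted with, runs a short countdown and then explodes.
; Interact reveals the hidden time display and starts a looping timer that updates the text and beeps on each tick.
; Once the count drops below zero, it clears the timer, spawns explosion particles and sound, activates the initially inactive BPFSCExplode component, and destroys itself.
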(event Custom|UpdateCountdown
  ;[0.15 0.15 0.15 0.5] Countdown du timer
  (bind _output_get (Variables|Default|SettimeRemaining (- (Variables|Default|GettimeRemaining) 1.0)))
  (if (< _output_get 0.0)
    (Utilities|Time|ClearandInvalidateTimerbyHandle (stale EventInteract _returnvalue))
    (Variables|Default|SetbombPosition (Transformation|GetWorldLocation (Variables|Default|GettimeWidgetRef)))
    (Effects|SpawnEmitteratLocation "/Game/Game/Actors/Dynamite/VFX/P_Explosion.P_Explosion" (Variables|Default|GetbombPosition))
    (Audio|PlaySoundatLocation "/Game/Game/Actors/Dynamite/Sounds/Explosion_Cue.Explosion_Cue" (Variables|Default|GetbombPosition) "0, 0, 0" 1.0 1.0 0.0 0 0 0 0)
    (Components|Activation|SetActive (Variables|Default|GetBP_FSC_Explode) true true)
    (Actor|DestroyActor)
    (else
      (Rendering|Components|TextRender|SetText (Variables|Default|GettimeWidgetRef) (Utilities|Text|ToText(Float) _output_get "HalfToEven"))
      (Variables|Default|SetbombPosition (Transformation|GetWorldLocation (Variables|Default|GetGC_BP_Dynamite)))
      (Audio|PlaySoundatLocation "/Game/Game/Actors/Dynamite/Sounds/Beep_Short__Cue.Beep_Short__Cue" (Variables|Default|GetbombPosition) "0, 0, 0" 1.0 1.0 0.0 0 0 0 0))))

(event EventBeginPlay
  (Components|Activation|SetActive (Variables|Default|GetBP_FSC_Explode) false false)
  (Rendering|SetVisibility (Variables|Default|GettimeWidgetRef) false false))

(event Collision|EventActorBeginOverlap
  (params (OtherActor :type Actor%20Object%20Reference)))

(event EventTick
  (params (DeltaSeconds :type Float%20%28single-precision%29)))

(event EventInteract
  (params (Actor :type Actor%20Object%20Reference))
  (Variables|Default|SettimeRemaining 3.0)
  (Rendering|SetVisibility (Variables|Default|GettimeWidgetRef) true false)
  ;[0.15 0.15 0.15 0.5] Countdown du timer
  (bind _returnvalue (Utilities|Time|SetTimerbyEvent (delegate Custom|UpdateCountdown) 1.0 true)))

(fn ConstructionScript)