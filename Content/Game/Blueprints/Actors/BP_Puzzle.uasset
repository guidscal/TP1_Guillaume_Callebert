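; Interactable puzzle actor that switches from an incomplete to a completed state and records that progress in the game.
; BeginPlay shows the incomplete component and hides both the completed one and the interaction prompt.
; Interact swaps the two components, plays a 2D sound and sets the Lv1Ch2 flag on BP_GameInstance.
; A sphere collision toggles the prompt widget on any overlap begin or end, without filtering the overlapping actor.
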(event OnComponentBeginOverlap(SphereCollision)
  (params (OverlappedComponent :type Primitive%20Component%20Object%20Reference) (OtherActor :type Actor%20Object%20Reference) (OtherComp :type Primitive%20Component%20Object%20Reference) (OtherBodyIndex :type Integer) (bFromSweep :type Boolean) (SweepResult :type Hit%20Result%20Structure%20%28by%20ref%29))
  ;[0.15 0.15 0.15 0.5] Interact Prompt
  (Rendering|SetVisibility (Variables|Default|GetWidgetTextInteraction) true false))

(event OnComponentEndOverlap(SphereCollision)
  (params (OverlappedComponent :type Primitive%20Component%20Object%20Reference) (OtherActor :type Actor%20Object%20Reference) (OtherComp :type Primitive%20Component%20Object%20Reference) (OtherBodyIndex :type Integer))
  ;[0.15 0.15 0.15 0.5] Interact Prompt
  (Rendering|SetVisibility (Variables|Default|GetWidgetTextInteraction) false false))

(event EventBeginPlay
  (bind _puzzlecomplete (Variables|Default|GetPuzzleComplete))
  (bind _puzzleincomplete (Variables|Default|GetPuzzleIncomplete))
  ;[0.15 0.15 0.15 0.5] Faire afficher le bon etat au depart
  (Components|Activation|SetActive _puzzlecomplete false false)
  (Rendering|SetVisibility _puzzlecomplete false false)
  (Components|Activation|SetActive _puzzleincomplete true false)
  (Rendering|SetVisibility _puzzleincomplete true false)
  (Rendering|SetVisibility (Variables|Default|GetWidgetTextInteraction) false false))

(event EventInteract
  (params (Actor :type Actor%20Object%20Reference))
  (bind _puzzlecomplete (Variables|Default|GetPuzzleComplete))
  (bind _puzzleincomplete (Variables|Default|GetPuzzleIncomplete))
  ;[0.15 0.15 0.15 0.5] Basculer etat quand interaction
  (Components|Activation|SetActive _puzzlecomplete true false)
  (Rendering|SetVisibility _puzzlecomplete true false)
  (Audio|PlaySound2D "/Game/Game/Audio/SFX/S_puzzle_Cue.S_puzzle_Cue" 1.0 1.0 0.0 0 0)
  (Components|Activation|SetActive _puzzleincomplete false false)
  (Rendering|SetVisibility _puzzleincomplete false false)
  (bind _asbp_game_instance (Utilities|Casting|CastToBP_GameInstance (Game|GetGameInstance)))
  (Variables|/Game/Game/Blueprints/GameInstance/BP_GameInstance.BP_GameInstance_C|SetLv1Ch2 _asbp_game_instance true))

(fn ConstructionScript)