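; BP_Scarabe is an interactable scarab actor that rotates through four orientations, likely as a puzzle piece.
; Each Interact call turns ScarabeFix a quarter turn and advances ScarabeState, wrapping back to the first state after the fourth, then plays a 2D sound.
; A sphere collision shows the interaction text widget on overlap and hides it on exit; the widget starts hidden.
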(event OnComponentBeginOverlap(SphereCollision)
  (params (OverlappedComponent :type Primitive%20Component%20Object%20Reference) (OtherActor :type Actor%20Object%20Reference) (OtherComp :type Primitive%20Component%20Object%20Reference) (OtherBodyIndex :type Integer) (bFromSweep :type Boolean) (SweepResult :type Hit%20Result%20Structure%20%28by%20ref%29))
  (Rendering|SetVisibility (Variables|Default|GetWidgetTextInteraction) true false))

(event OnComponentEndOverlap(SphereCollision)
  (params (OverlappedComponent :type Primitive%20Component%20Object%20Reference) (OtherActor :type Actor%20Object%20Reference) (OtherComp :type Primitive%20Component%20Object%20Reference) (OtherBodyIndex :type Integer))
  (Rendering|SetVisibility (Variables|Default|GetWidgetTextInteraction) false false))

(event EventBeginPlay
  (Rendering|SetVisibility (Variables|Default|GetWidgetTextInteraction) false false))

(event Collision|EventActorBeginOverlap
  (params (OtherActor :type Actor%20Object%20Reference)))

(event EventTick
  (params (DeltaSeconds :type Float%20%28single-precision%29)))

(event EventInteract
  (params (Actor :type Actor%20Object%20Reference))
  (if (< (Variables|Components|GetScarabeState) 4)
    (Transformation|AddLocalRotation (Variables|Default|GetScarabeFix) "0.000000,90.000000,0.000000" false false)
    (Variables|Components|SetScarabeState (+ (Variables|Components|GetScarabeState) 1))
    (else
      (Variables|Components|SetScarabeState 1)
      (Transformation|AddLocalRotation (Variables|Default|GetScarabeFix) "0.000000,-270.000000,0.000000" false false)))
  (Audio|PlaySound2D "/Game/Game/Audio/SFX/S_scarabe_Cue.S_scarabe_Cue" 1.0 1.0 0.0 0 0))

(fn ConstructionScript)