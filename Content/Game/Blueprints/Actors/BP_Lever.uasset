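; BP_Lever is an end-game lever that starts hidden at zero scale and appears once Level 1 is complete.
; Tick polls the GameInstance's Level1Complete flag, then after a delay runs a timeline that lerps the lever and base up to full size.
; Sphere overlap toggles an interaction text widget.
; Interact plays a pull sound, calls the end-game event, sets GameComplete on the GameInstance and rotates the lever.
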(event OnComponentBeginOverlap(SphereCollision)
  (params (OverlappedComponent :type Primitive%20Component%20Object%20Reference) (OtherActor :type Actor%20Object%20Reference) (OtherComp :type Primitive%20Component%20Object%20Reference) (OtherBodyIndex :type Integer) (bFromSweep :type Boolean) (SweepResult :type Hit%20Result%20Structure%20%28by%20ref%29))
  (Rendering|SetVisibility (Variables|Default|GetWidgetTextInteraction) true false))

(event OnComponentEndOverlap(SphereCollision)
  (params (OverlappedComponent :type Primitive%20Component%20Object%20Reference) (OtherActor :type Actor%20Object%20Reference) (OtherComp :type Primitive%20Component%20Object%20Reference) (OtherBodyIndex :type Integer))
  (Rendering|SetVisibility (Variables|Default|GetWidgetTextInteraction) false false))

(event EventBeginPlay
  (Transformation|SetWorldScale3D (Variables|Default|GetLever) "0, 0, 0")
  (bind _asbp_game_instance (Utilities|Casting|CastToBP_GameInstance (Game|GetGameInstance)))
  (Variables|Default|SetAs%20BP%20Game%20Instance _asbp_game_instance)
  (Rendering|SetVisibility (Variables|Default|GetWidgetTextInteraction) false false))

(event Collision|EventActorBeginOverlap
  (params (OtherActor :type Actor%20Object%20Reference)))

(event EventTick
  (params (DeltaSeconds :type Float%20%28single-precision%29))
  (bind _lever (Variables|Default|GetLever))
  (if (Variables|/Game/Game/Blueprints/GameInstance/BP_GameInstance.BP_GameInstance_C|GetLevel1Complete (Variables|Default|GetAs%20BP%20Game%20Instance))
    (Utilities|FlowControl|Delay 3.0)
    (bind _smooth (Timeline|Smooth Play)
      (:Update
        (Transformation|SetWorldScale3D _lever (Math|Vector|Lerp(Vector) (Transformation|GetWorldScale _lever) "1.000000,1.000000,1.000000" _smooth))))))

(event EventInteract
  (params (Actor :type Actor%20Object%20Reference))
  (Audio|PlaySound2D "/Game/Game/Audio/SFX/S_leverPull_Cue.S_leverPull_Cue" 1.0 1.0 0.0 0 0)
  (Default|CallEventEndGame)
  (Variables|/Game/Game/Blueprints/GameInstance/BP_GameInstance.BP_GameInstance_C|SetGameComplete (Variables|Default|GetAs%20BP%20Game%20Instance) true)
  (Transformation|SetRelativeRotation (Variables|Default|GetLever) "0.000000,0.000000,55.000000" false false))

(fn ConstructionScript)