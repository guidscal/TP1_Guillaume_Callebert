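; BP_ScarabeChallenge is a puzzle actor for level 1, challenge 1, solved when three scarabs are in their correct positions.
; Every Tick it reads the state of its three BP_Scarabe child actors and compares each to its expected value.
; It writes the result to Lv1Ch1 on BP_GameInstance, so completion is not latched and reverts when any scarab leaves its correct state.
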(event EventBeginPlay)

(event Collision|EventActorBeginOverlap
  (params (OtherActor :type Actor%20Object%20Reference)))

(event EventTick
  (params (DeltaSeconds :type Float%20%28single-precision%29))
  ;[0.15 0.15 0.15 0.5] Creer les variables pour les 3 scarabes
  (bind _asbp_scarabe (Utilities|Casting|CastToBP_Scarabe (Variables|/Script/Engine.ChildActorComponent|GetChildActor (Variables|Default|GetBP_Scarabe1))))
  (Variables|Default|SetScarabe1State (Variables|/Game/Game/Blueprints/Actors/BP_Scarabe.BP_Scarabe_C|GetScarabeState _asbp_scarabe))
  (bind _asbp_scarabe_2 (Utilities|Casting|CastToBP_Scarabe (Variables|/Script/Engine.ChildActorComponent|GetChildActor (Variables|Default|GetBP_Scarabe2))))
  (Variables|Default|SetScarabe2State (Variables|/Game/Game/Blueprints/Actors/BP_Scarabe.BP_Scarabe_C|GetScarabeState _asbp_scarabe_2))
  (bind _asbp_scarabe_3 (Utilities|Casting|CastToBP_Scarabe (Variables|/Script/Engine.ChildActorComponent|GetChildActor (Variables|Default|GetBP_Scarabe3))))
  (Variables|Default|SetScarabe3State (Variables|/Game/Game/Blueprints/Actors/BP_Scarabe.BP_Scarabe_C|GetScarabeState _asbp_scarabe_3))
  ;[0.15 0.15 0.15 0.5] Valider si bonne reponse
  (if (Math|Boolean|ANDBoolean (== (Variables|Default|GetScarabe1State) (Variables|Default|GetScarabe1CorrectPos)) (== (Variables|Default|GetScarabe2State) (Variables|Default|GetScarabe2CorrectPos)) (== (Variables|Default|GetScarabe3State) (Variables|Default|GetScarabe3CorrectPos)))
    ;[0.15 0.15 0.15 0.5] Changer variable pour enigme complete
    (bind _asbp_game_instance (Utilities|Casting|CastToBP_GameInstance (Game|GetGameInstance)))
    (Variables|/Game/Game/Blueprints/GameInstance/BP_GameInstance.BP_GameInstance_C|SetLv1Ch1 _asbp_game_instance true)
    (else
      (bind _asbp_game_instance_2 (Utilities|Casting|CastToBP_GameInstance (Game|GetGameInstance)))
      (Variables|/Game/Game/Blueprints/GameInstance/BP_GameInstance.BP_GameInstance_C|SetLv1Ch1 _asbp_game_instance_2 false))))

(fn ConstructionScript)